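; Interactable padlocked chest for a code puzzle.
; Interaction locks and hides the player, blends the view to the chest, and shows the padlock widget, or the enigma widget once CodeTrouver is set, creating each only once.
; The ouverture event hides the padlock, then chains two timelines to rotate the latch and then the lid.
; Surbriance briefly applies an outline overlay to the lid while the chest is unused.
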(event `/Game/BP/BPI/BPI_Interaction.Interaction`
  (bind _player (`self.Player`))
  (set `self.Use` true)
  (set `PlayerController.bShowMouseCursor` true (`GameplayStatics.GetPlayerController` 0))
  (set `/Game/BP/Player/BP_Player.CanInteractOVer` false _player)
  (set `/Game/BP/Player/BP_Player.CanMove` false _player)
  (set `/Game/BP/Player/BP_Player.CanLook` false _player)
  (`self.SetActorHiddenInGame` _player true)
  (if (`self.CodeTrouver`)
    (if (`self.PremiereFOis2`)
      (bind _returnvalue (`|CreateWidget` "/Game/BP/Inspection/WG_Inspect/WG_Enigme.WG_Enigme_C"))
      (bind _output_get (set `self.WG_Ref` _returnvalue))
      (`UserWidget.AddToViewport` _output_get 0)
      (set `self.PremiereFOis2` false)
      (else
        (`Widget.SetVisibility` (`self.Wg_Ref`) "Visible")))
    (`PlayerController.SetViewTargetWithBlend` (`GameplayStatics.GetPlayerController` 0) self 0.0 "VTBlend_Linear" 0.0 false)
    (else
      (if (`self.Premierefois`)
        (bind _returnvalue_2 (`|CreateWidget` "/Game/BP/Cadena/WG_CadenasAffi.WG_CadenasAffi_C"))
        (`UserWidget.AddToViewport` _returnvalue_2 0)
        (set `self.Premierefois` false)
        (else
          (`Widget.SetVisibility` _returnvalue_2 "Visible")))
      ;[1 1 1] Switch de cam
      (`PlayerController.SetViewTargetWithBlend` (`GameplayStatics.GetPlayerController` 0) self 0.0 "VTBlend_Linear" 0.0 false))))

(event `ouverture`
  (`SceneComponent.SetVisibility` (`self.cadenas`) false false)
  (bind (_direction _newtrack_0) (`Timeline|Timeline`)
    (:`Update`
      (`SceneComponent.K2_SetRelativeRotation` (`self.LockCoffre`) (`KismetMathLibrary.MakeRotator` 0.0 (`KismetMathLibrary.Lerp` 0.0 120.0 _newtrack_0)) false false))
    (:`Finished`
      (bind (_direction_2 _newtrack_0_2 _newtrack_1) (`Timeline|Timeline_0`)
        (:`Update`
          (`SceneComponent.K2_SetRelativeRotation` (`self.HautCoffre`) (`KismetMathLibrary.MakeRotator` 0.0 (`KismetMathLibrary.Lerp` 0.0 120.0 _newtrack_1)) false false))))))

(event `/Game/BP/BPI/BPI_Surbriance.Surbriance`
  (params (Board_Component :type "ActorComponent Object Reference"))
  (bind _hautcoffre (`self.HautCoffre`))
  (if (not (`self.Use`))
    (`MeshComponent.SetOverlayMaterial` _hautcoffre "/Game/Assets/Material/OutlineMat/M_Outline_Inst1.M_Outline_Inst1")
    (`KismetSystemLibrary.Delay` 0.5)
    (`MeshComponent.SetOverlayMaterial` _hautcoffre null)))

(fn `UserConstructionScript`)