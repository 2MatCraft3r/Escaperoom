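; Interactive book actor, the second book in a secret-code puzzle driven by BPCodeSecret.
; On first Interaction it increments the shared Compteur, stores that value as its order in Livre02, and plays a timeline tilting Livre01; the DejaUse2 flag blocks repeats.
; Revers1 plays a separate timeline in reverse to rotate Livre01 and LettreS in relative space, without clearing the flag.
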(event `Revers1`
  (bind (_direction _newtrack_0) (`Timeline|Timeline_0` :!via `Reverse`)
    (:`Update`
      (`SceneComponent.K2_SetRelativeRotation` (`self.Livre01`) (`KismetMathLibrary.MakeRotator` (`KismetMathLibrary.Lerp` 0.0 -15.0 _newtrack_0)) false false)
      (`SceneComponent.K2_SetRelativeRotation` (`self.lettreS`) (`KismetMathLibrary.MakeRotator` (`KismetMathLibrary.Lerp` 0.0 15.0 _newtrack_0)) false false))))

(event `/Game/BP/BPI/BPI_Interaction.Interaction`
  (bind _bp_codesecret (`self.BP_CodeSecret`))
  (bind _returnvalue (+ (`/Game/BP/CodeSecret/BP_CodeSecret.Compteur` _bp_codesecret) 1.0))
  (if (`self.DejaUse2`)
    (`KismetSystemLibrary.PrintString` "deja Use 2")
    (else
      (set `self.DejaUse2` true)
      (`KismetSystemLibrary.PrintString` "Livre2")
      (bind _output_get (set `self.Livre02` _returnvalue))
      (set `/Game/BP/CodeSecret/BP_CodeSecret.Compteur` _returnvalue _bp_codesecret)
      (`KismetSystemLibrary.PrintString` (`KismetStringLibrary.Conv_DoubleToString` _output_get))
      (bind (_direction _newtrack_0) (`Timeline|Timeline`)
        (:`Update`
          (`SceneComponent.K2_SetWorldRotation` (`self.Livre01`) (`KismetMathLibrary.MakeRotator` (`KismetMathLibrary.Lerp` 0.0 15.0 _newtrack_0)) false false))))))

(fn `UserConstructionScript`)