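; BP_CodeLivre04 is an interactable book, one input of a secret-code puzzle managed by BPCodeSecret.
; Interaction works once, recording the book's press order from the shared Compteur, then pitching it via timeline and calling VoirSiCodeBon on every update.
; Reverse04 runs a separate timeline in reverse on yaw, with a Reset flag blocking the tilt meanwhile, but leaves DejaUse4 set.
; Surbriance briefly applies an outline overlay as a highlight.
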(event `Reverse04`
  (set `self.reset` true)
  (bind (_direction _newtrack_0) (`Timeline|Timeline_0` :!via `Reverse`)
    (:`Update`
      (`SceneComponent.K2_SetRelativeRotation` (`self.Livre01`) (`KismetMathLibrary.MakeRotator` 0.0 0.0 (`KismetMathLibrary.Lerp` 0.0 -15.0 _newtrack_0)) false false))
    (:`Finished`
      (set `self.reset` false))))

(event `/Game/BP/BPI/BPI_Interaction.Interaction`
  (bind _bp_codesecret (`self.BP_CodeSecret`))
  (bind _returnvalue (+ (`/Game/BP/CodeSecret/BP_CodeSecret.Compteur` _bp_codesecret) 1.0))
  (if (`self.DejaUse4`)
    (`KismetSystemLibrary.PrintString` "deja utiliser")
    (else
      (set `self.DejaUse4` true)
      (`KismetSystemLibrary.PrintString` "Livre1")
      (bind _output_get (set `self.Livre4` _returnvalue))
      (set `/Game/BP/CodeSecret/BP_CodeSecret.Compteur` _returnvalue _bp_codesecret)
      (`KismetSystemLibrary.PrintString` (`KismetStringLibrary.Conv_DoubleToString` _output_get))
      (if (not (`self.reset`))
        (bind (_direction _newtrack_0) (`Timeline|Timeline` :!via `PlayFromStart`)
          (:`Update`
            (`SceneComponent.K2_SetRelativeRotation` (`self.Livre01`) (`KismetMathLibrary.MakeRotator` 0.0 (`KismetMathLibrary.Lerp` 0.0 -15.0 _newtrack_0)) false false)
            (`/Game/BP/CodeSecret/BP_CodeSecret.VoirSiCodeBon` (`self.BP_CodeSecret`))))))))

(event `/Game/BP/BPI/BPI_Surbriance.Surbriance`
  (bind _livre01 (`self.Livre01`))
  (`MeshComponent.SetOverlayMaterial` _livre01 "/Game/Assets/Material/OutlineMat/M_Outline_Inst1.M_Outline_Inst1")
  (`KismetSystemLibrary.Delay` 0.5)
  (`MeshComponent.SetOverlayMaterial` _livre01 "/Game/Assets/Material/OutlineMat/Clear.Clear"))

(fn `UserConstructionScript`)