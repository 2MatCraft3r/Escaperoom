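; Player character using Enhanced Input for camera-relative movement and look, interaction with world actors, and drawing on a board.
; Each tick a box trace from the head socket along the camera sends SurbrianceMessage to the hit actor; Interact runs the same trace, with a delay gate, for InteractionMessage.
; Draw traces around the cursor's hit point and passes collision UV and brush settings to BP_Tableau.
; Montage jump and speed-switch logic is unwired.
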(event `self.ReceiveBeginPlay`
  (bind _asplayer_controller (cast `PlayerController` (`self.GetController`)))
  (`EnhancedInputSubsystemInterface.AddMappingContext` (pcsubsystem `EnhancedInputLocalPlayerSubsystem` _asplayer_controller) "/Game/Inputs/IMC_Player.IMC_Player" 0 (struct))
  (set `CharacterMovementComponent.MaxWalkSpeed` 250.0 (`self.CharacterMovement`)))

(event `EnhancedInput|/Game/Inputs/Actions/IA_Move`
  (params (ActionValue :type "Vector2D Structure") (ElapsedSeconds :type "Float (double-precision)") (TriggeredSeconds :type "Float (double-precision)") (InputAction :type "InputAction Object Reference" :default "/Game/Inputs/Actions/IA_Move.IA_Move"))
  (bind (_returnvalue_roll _returnvalue_pitch _returnvalue_yaw) (`KismetMathLibrary.BreakRotator` (`SceneComponent.K2_GetComponentRotation` (`self.CameraPlayer`))))
  (:`Triggered`
    (if (`self.CanMove`)
      (`self.AddMovementInput` (`KismetMathLibrary.GetForwardVector` (`KismetMathLibrary.MakeRotator` 0.0 0.0 _returnvalue_yaw)) ActionValue_X)
      (`self.AddMovementInput` (`KismetMathLibrary.GetRightVector` (`KismetMathLibrary.MakeRotator` 0.0 0.0 _returnvalue_yaw)) ActionValue_Y)))
  (:`Started`
    (set `self.Move` true))
  (:`Completed`
    (set `self.Move` false)))

(event `EnhancedInput|/Game/Inputs/Actions/IA_Look`
  (params (ActionValue :type "Vector2D Structure") (ElapsedSeconds :type "Float (double-precision)") (TriggeredSeconds :type "Float (double-precision)") (InputAction :type "InputAction Object Reference" :default "/Game/Inputs/Actions/IA_Look.IA_Look"))
  (:`Triggered`
    (if (`self.CanLook`)
      (`self.AddControllerYawInput` ActionValue_X)
      (`self.AddControllerPitchInput` ActionValue_Y))))

(event `EnhancedInput|/Game/Inputs/Actions/IA_Jump`
  (params (ActionValue :type Boolean) (ElapsedSeconds :type "Float (double-precision)") (TriggeredSeconds :type "Float (double-precision)") (InputAction :type "InputAction Object Reference" :default "/Game/Inputs/Actions/IA_Jump.IA_Jump")))

(event `Key|LeftShift`
  (params (Key :type "Key Structure")))

(event `self.OnLanded`
  (params (Hit :type "HitResult Structure (by ref)"))
  (set `self.bCanJump` true))

(event `EnhancedInput|/Game/Inputs/Actions/IA_Interact`
  (params (ActionValue :type Boolean) (ElapsedSeconds :type "Float (double-precision)") (TriggeredSeconds :type "Float (double-precision)") (InputAction :type "InputAction Object Reference" :default "/Game/Inputs/Actions/IA_Interact.IA_Interact"))
  (:`Triggered`
    (if (`self.CanInteractOVer`)
      (bind _asbp_player (cast `/Game/BP/Player/BP_Player` (`GameplayStatics.GetPlayerCharacter` 0)))
      (if (`self.CanIteractDelay`)
        (set `self.CanIteractDelay` false)
        (bind _returnvalue (`SceneComponent.GetSocketLocation` (`Character.Mesh` _asbp_player) "Head"))
        (bind _outhit (`KismetSystemLibrary.BoxTraceSingle` :`Start` _returnvalue :`End` (+ _returnvalue (* (`SceneComponent.GetForwardVector` (`/Game/BP/Player/BP_Player.CameraPlayer` _asbp_player)) 250.0)) :`HalfSize` (10.0 10.0 10.0) :`TraceChannel` "TraceTypeQuery1" :`DrawDebugType` "ForDuration"))
        (set `self.ActualActor` (`.HitActor` (`GameplayStatics.BreakHitResult` _outhit)))
        (message `/Game/BP/BPI/BPI_Interaction.Interaction` (`.HitActor` (`GameplayStatics.BreakHitResult` _outhit)))
        (`KismetSystemLibrary.Delay` 1.0)
        (set `self.CanIteractDelay` true)))))

(event `self.ReceiveTick`
  (params (DeltaSeconds :type "Float (single-precision)"))
  (bind _asbp_player (cast `/Game/BP/Player/BP_Player` (`GameplayStatics.GetPlayerCharacter` 0)))
  (bind _returnvalue (`SceneComponent.GetSocketLocation` (`Character.Mesh` _asbp_player) "Head"))
  (bind _outhit (`KismetSystemLibrary.BoxTraceSingle` _returnvalue (+ _returnvalue (* (`SceneComponent.GetForwardVector` (`/Game/BP/Player/BP_Player.CameraPlayer` _asbp_player)) 250.0)) (10.0 10.0 10.0) (struct) "TraceTypeQuery1"))
  (message `/Game/BP/BPI/BPI_Surbriance.Surbriance` (`.HitActor` (`GameplayStatics.BreakHitResult` _outhit)) (`.HitComponent` (`GameplayStatics.BreakHitResult` _outhit))))

(event `EnhancedInput|/Game/Inputs/Actions/IA_Draw`
  (params (ActionValue :type Boolean) (ElapsedSeconds :type "Float (double-precision)") (TriggeredSeconds :type "Float (double-precision)") (InputAction :type "InputAction Object Reference" :default "/Game/Inputs/Actions/IA_Draw.IA_Draw"))
  (bind _hitresult (`PlayerController.GetHitResultUnderCursorByChannel` (`GameplayStatics.GetPlayerController` 0) "TraceTypeQuery1" true))
  (:`Triggered`
    (if (`self.CanDraw`)
      (bind _outhit (`KismetSystemLibrary.LineTraceSingle` :`Start` (`KismetMathLibrary.MakeVector` (+ (.x (`.ImpactPoint` (`GameplayStatics.BreakHitResult` _hitresult))) 100.0) (.y (`.ImpactPoint` (`GameplayStatics.BreakHitResult` _hitresult))) (.z (`.ImpactPoint` (`GameplayStatics.BreakHitResult` _hitresult)))) :`End` (`KismetMathLibrary.MakeVector` (+ (.x (`.ImpactPoint` (`GameplayStatics.BreakHitResult` _hitresult))) -100.0) (.y (`.ImpactPoint` (`GameplayStatics.BreakHitResult` _hitresult))) (.z (`.ImpactPoint` (`GameplayStatics.BreakHitResult` _hitresult)))) :`TraceChannel` "TraceTypeQuery1" :`bTraceComplex` true :`DrawDebugType` "ForDuration"))
      (bind _asbp_tableau (cast `/Game/BP/TableauDessin/BP_Tableau` (`.HitActor` (`GameplayStatics.BreakHitResult` _outhit)))
        (:`then`
          (`/Game/BP/TableauDessin/BP_Tableau.Draw` _asbp_tableau (`GameplayStatics.FindCollisionUV` _outhit) (`self.BrushTexture`) (`self.brushSize`)))
        (:`CastFailed`
          (`KismetSystemLibrary.PrintString` "Faild"))))))

(fn `UserConstructionScript`)