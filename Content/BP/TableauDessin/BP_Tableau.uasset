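; Drawing board actor that the player interacts with to enter and leave a drawing mode.
; Interaction uses a FlipFlop to switch the view between board and character, toggling the mouse cursor, player visibility and the player's camera and draw flags.
; Draw is an unfinished brush stamp on the Ren_Pinceau render target: it draws at a fixed corner position, sets no material and never ends the canvas draw.
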(event `/Game/BP/BPI/BPI_Interaction.Interaction`
  (bind _player (`self.Player`))
  (bind _player_2 (`self.Player`))
  (`/Engine/EditorBlueprintResources/StandardMacros.FlipFlop`
    (:`A`
      ;[1 1 1] Switch de cam
      (`PlayerController.SetViewTargetWithBlend` (`GameplayStatics.GetPlayerController` 0) self 0.0 "VTBlend_Linear" 0.0 false)
      (set `PlayerController.bShowMouseCursor` true (`GameplayStatics.GetPlayerController` 0))
      (set `/Game/BP/Player/BP_Player.CamPersActive` false _player_2)
      (set `/Game/BP/Player/BP_Player.CanDraw` true _player_2)
      (`self.SetActorHiddenInGame` _player_2 true))
    (:`B`
      (`PlayerController.SetViewTargetWithBlend` (`GameplayStatics.GetPlayerController` 0) (`GameplayStatics.GetPlayerCharacter` 0) 0.0 "VTBlend_Linear" 0.0 false)
      (set `PlayerController.bShowMouseCursor` false (`GameplayStatics.GetPlayerController` 0))
      (set `/Game/BP/Player/BP_Player.CamPersActive` true _player)
      (set `/Game/BP/Player/BP_Player.CanDraw` false _player)
      (`self.SetActorHiddenInGame` _player false))))

(event `Draw`
  (`KismetSystemLibrary.PrintString` "DebutDraw")
  (bind (_canvas _size) (`KismetRenderingLibrary.BeginDrawCanvasToRenderTarget` "/Game/BP/TableauDessin/Ren_Pinceau.Ren_Pinceau"))
  (`Canvas.K2_DrawMaterial` _canvas null (- (* _size (0.0 0.0)) (/ (`self.BrushSize`) 2.0)) (0.0 0.0) (0.0 0.0) (1.0 1.0) 0.0 (0.5 0.5)))

(fn `UserConstructionScript`)