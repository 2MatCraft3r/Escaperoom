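; BP_IndiceOrange is an interactable actor that opens the orange clue (indice) inspection widget for the player.
; Its Interaction event creates WG_IndiceOrange on first use, caches it, and makes it visible again on later uses.
; It then shows the mouse cursor, disables the BP_Player movement, look and interaction-over flags, and hides the player character.
; Closing the widget and restoring the player are not handled here.
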(event `/Game/BP/BPI/BPI_Interaction.Interaction`
  (if (`self.Premierefois`)
    (set `self.PremiereFois` false)
    (bind _returnvalue (`|CreateWidget` "/Game/BP/Inspection/WG_Inspect/WG_IndiceOrange.WG_IndiceOrange_C"))
    (bind _output_get (set `self.WG_Ref` _returnvalue))
    (`UserWidget.AddToPlayerScreen` _output_get 0)
    (else
      (`Widget.SetVisibility` (`self.WG_Ref`) "Visible")))
  (set `PlayerController.bShowMouseCursor` true (`GameplayStatics.GetPlayerController` 0))
  (bind _asbp_player (cast `/Game/BP/Player/BP_Player` (`GameplayStatics.GetPlayerCharacter` 0)))
  (set `/Game/BP/Player/BP_Player.CanInteractOVer` false _asbp_player)
  (set `/Game/BP/Player/BP_Player.CanMove` false _asbp_player)
  (set `/Game/BP/Player/BP_Player.CanLook` false _asbp_player)
  (`self.SetActorHiddenInGame` (`GameplayStatics.GetPlayerCharacter` 0) true))

(fn `UserConstructionScript`)