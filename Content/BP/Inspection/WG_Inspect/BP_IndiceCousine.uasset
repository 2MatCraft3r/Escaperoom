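; BP_IndiceCousine is an interactable clue actor that opens its inspection widget.
; On Interaction it adds WG_IndiceCousine to the player screen and shows the mouse cursor.
; It then disables interaction, movement and look on BP_Player and hides the player character in game.
; Nothing in this Blueprint restores those states or removes the widget.
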(event `self.Interaction`
  (bind _returnvalue (`|CreateWidget` "/Game/BP/Inspection/WG_Inspect/WG_IndiceCousine.WG_IndiceCousine_C"))
  (`UserWidget.AddToPlayerScreen` _returnvalue 0)
  (set `PlayerController.bShowMouseCursor` true (`GameplayStatics.GetPlayerController` 0))
  (bind _asbp_player (cast `/Game/BP/Player/BP_Player` (`GameplayStatics.GetPlayerCharacter` 0)))
  (set `/Game/BP/Player/BP_Player.CanInteractOVer` false _asbp_player)
  (set `/Game/BP/Player/BP_Player.CanMove` false _asbp_player)
  (set `/Game/BP/Player/BP_Player.CanLook` false _asbp_player)
  (`self.SetActorHiddenInGame` (`GameplayStatics.GetPlayerCharacter` 0) true))

(fn `UserConstructionScript`)