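; BP_Indices is an interactable clue book actor that opens a hint widget for the player.
; On BeginPlay it creates WG_Indices, then Interaction adds it to the viewport the first time, re-shows it afterwards, and calls its sheet display.
; Interaction also shows the cursor, locks movement, look and further interaction, and hides the player character.
; Surbriance briefly flashes an outline overlay material on the book.
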(event `self.ReceiveBeginPlay`
  (bind _returnvalue (`|CreateWidget` "/Game/BP/Inspection/WG_Inspect/WG_Indices.WG_Indices_C"))
  (set `self.RefIndices` _returnvalue))

(event `/Game/BP/BPI/BPI_Interaction.Interaction`
  (bind _player (`self.Player`))
  (if (`self.PremiereFois`)
    (set `self.PremiereFois` false)
    (`UserWidget.AddToViewport` (`self.RefIndices`) 0)
    (else
      (`Widget.SetVisibility` (`self.RefIndices`) "Visible")))
  (set `PlayerController.bShowMouseCursor` true (`GameplayStatics.GetPlayerController` 0))
  (`/Game/BP/Inspection/WG_Inspect/WG_Indices.AffichaFeuile` (`self.RefIndices`))
  (set `/Game/BP/Player/BP_Player.CanMove` false _player)
  (set `/Game/BP/Player/BP_Player.CanInteractOVer` false _player)
  (set `/Game/BP/Player/BP_Player.CanLook` false _player)
  (`self.SetActorHiddenInGame` (`GameplayStatics.GetPlayerCharacter` 0) true))

(event `/Game/BP/BPI/BPI_Surbriance.Surbriance`
  (`MeshComponent.SetOverlayMaterial` (`self.LivresIndices`) "/Game/Assets/Material/OutlineMat/M_Outline_Inst1.M_Outline_Inst1")
  (`KismetSystemLibrary.Delay` 0.5)
  (`MeshComponent.SetOverlayMaterial` (`self.LivresIndices`) null))

(fn `UserConstructionScript`)