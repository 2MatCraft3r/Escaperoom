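; BP_LivreCode01 is the first book in a secret-code puzzle, apparently order-based, and can be used only once.
; On Interaction it sets DejaUse, increments the shared Compteur on BPCodeSecret and stores the new count in Livre1 as its position in the sequence.
; It then calls VoirSiCodeBon on BPCodeSecret to check the code, printing debug strings along the way.
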(event `self.ReceiveBeginPlay`)

(event `/Game/BPI_Interaction.Interaction`
  (bind _bp_codesecret (`self.BP_CodeSecret`))
  (bind _returnvalue (+ (`/Game/BP_CodeSecret.Compteur` _bp_codesecret) 1.0))
  (if (`self.DejaUse`)
    (`KismetSystemLibrary.PrintString` "deja utiliser")
    (else
      (set `self.DejaUse` true)
      (`KismetSystemLibrary.PrintString` "Livre1")
      (bind _output_get (set `self.Livre1` _returnvalue))
      (set `/Game/BP_CodeSecret.Compteur` _returnvalue _bp_codesecret)
      (`KismetSystemLibrary.PrintString` (`KismetStringLibrary.Conv_DoubleToString` _output_get))
      (`/Game/BP_CodeSecret.VoirSiCodeBon` (`self.BP_CodeSecret`)))))

(fn `UserConstructionScript`)