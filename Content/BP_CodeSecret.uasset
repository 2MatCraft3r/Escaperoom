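; BP_CodeSecret checks a four-book order puzzle that opens a secret door.
; VoirSiCodeBon reads a value from each of the four book Blueprints and calls OuverturePorte on BPPorteSecret when they match the expected one-to-four sequence.
; If all books are set but the order is wrong, it plays a ping and resets the counter, book values and used flags.
; Incomplete attempts are left untouched.
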(event `self.ReceiveBeginPlay`
  (set `self.Compteur` 0.0))

(event `VoirSiCodeBon`
  (bind _bp_livre2 (`self.BP_Livre2`))
  (bind _bp_livre3 (`self.BP_Livre3`))
  (bind _bp_livre4 (`self.BP_Livre4`))
  (bind _bp_livre1 (`self.BP_Livre1`))
  (bind _livre1 (`/Game/BP_LivreCode01.Livre1` (`self.BP_Livre1`)))
  (bind _livre02 (`/Game/BP_LivreCode02.Livre02` (`self.BP_Livre2`)))
  (bind _livre03 (`/Game/BP_LivreCode03.Livre03` (`self.BP_Livre3`)))
  (bind _livre04 (`/Game/BP_LivreCode04.Livre04` (`self.BP_Livre4`)))
  (if (and (== _livre1 1.0) (== _livre02 2.0) (== _livre03 3.0) (== _livre04 4.0))
    (`/Game/BP_PorteSecrete.OuverturePorte` (`self.BP_PorteSecret`))
    (elif (not (or (== _livre1 0.0) (== _livre02 0.0) (== _livre03 0.0) (== _livre04 0.0)))
      (`GameplayStatics.PlaySound2D` "/Engine/EngineSounds/1kSineTonePing.1kSineTonePing" 1.0 1.0 0.0 null null)
      (set `self.Compteur` 0.0)
      (set `/Game/BP_LivreCode01.Livre1` 0.0 _bp_livre1)
      (set `/Game/BP_LivreCode01.DejaUse` false _bp_livre1)
      (set `/Game/BP_LivreCode02.Livre02` 0.0 _bp_livre2)
      (set `/Game/BP_LivreCode02.DejaUse2` false _bp_livre2)
      (set `/Game/BP_LivreCode03.Livre03` 0.0 _bp_livre3)
      (set `/Game/BP_LivreCode03.DejaUse3` false _bp_livre3)
      (set `/Game/BP_LivreCode04.Livre04` 0.0 _bp_livre4)
      (set `/Game/BP_LivreCode04.DejaUse4` false _bp_livre4))))

(fn `UserConstructionScript`)