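; BP_AmbianceSong is an ambiance music actor that plays and switches tracks on one Audio component.
; BeginPlay sets the first song and, after a delay, raises its volume with a timeline.
; Music2, Music3 and music4 each use paired timelines to fade out and bring in another track.
; Stop, track swap, fade-in restart and Play all hang off timeline Update pins, so they repeat every update.
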(event `self.ReceiveBeginPlay`
  (bind _audio (`self.Audio`))
  (`AudioComponent.SetSound` _audio "/Game/Song/Mathematical_Mystery.Mathematical_Mystery")
  (`KismetSystemLibrary.Delay` 3.0)
  (bind (_direction _newtrack_0) (`Timeline|Timeline`)
    (:`Update`
      (`AudioComponent.SetVolumeMultiplier` _audio (`KismetMathLibrary.Lerp` 0.0 0.5 _newtrack_0))
      (`AudioComponent.Play` _audio 0.0))))

(event `Music2`
  (bind _audio (`self.Audio`))
  (bind (_direction _newtrack_0) (`Timeline|Timeline_1` :!via `PlayFromStart`)
    (:`Update`
      (`AudioComponent.SetVolumeMultiplier` _audio (`KismetMathLibrary.Lerp` 0.7 0.0 _newtrack_0))
      (`AudioComponent.Stop` _audio)
      (`AudioComponent.SetSound` _audio "/Game/Song/Mathematical_Mystery__1_.Mathematical_Mystery__1_")
      (bind (_direction_2 _newtrack_0_2) (`Timeline|Timeline_0` :!via `PlayFromStart`)
        (:`Update`
          (`AudioComponent.SetVolumeMultiplier` _audio (`KismetMathLibrary.Lerp` 0.0 0.5 _newtrack_0_2))
          (`AudioComponent.Play` _audio 0.0))))))

(event `Music3`
  (bind _audio (`self.Audio`))
  (bind (_direction _newtrack_0) (`Timeline|Timeline_3` :!via `PlayFromStart`)
    (:`Update`
      (`AudioComponent.SetVolumeMultiplier` _audio (`KismetMathLibrary.Lerp` 0.7 0.0 _newtrack_0))
      (`AudioComponent.Stop` _audio)
      (`AudioComponent.SetSound` _audio "/Game/Song/The_Clock_s_Equation.The_Clock_s_Equation")
      (bind (_direction_2 _newtrack_0_2) (`Timeline|Timeline_2` :!via `PlayFromStart`)
        (:`Update`
          (`AudioComponent.SetVolumeMultiplier` _audio (`KismetMathLibrary.Lerp` 0.0 0.5 _newtrack_0_2))
          (`AudioComponent.Play` _audio 0.0))))))

(event `music4`
  (bind _audio (`self.Audio`))
  (bind (_direction _newtrack_0) (`Timeline|Timeline_5` :!via `PlayFromStart`)
    (:`Update`
      (`AudioComponent.SetVolumeMultiplier` _audio (`KismetMathLibrary.Lerp` 0.7 0.0 _newtrack_0))
      (`AudioComponent.Stop` _audio)
      (`AudioComponent.SetSound` _audio "/Game/Song/Project_3-NotAK.Project_3-NotAK")
      (bind (_direction_2 _newtrack_0_2) (`Timeline|Timeline_4` :!via `PlayFromStart`)
        (:`Update`
          (`AudioComponent.SetVolumeMultiplier` _audio (`KismetMathLibrary.Lerp` 0.0 0.5 _newtrack_0_2))
          (`AudioComponent.Play` _audio 0.0))))))

(fn `UserConstructionScript`)